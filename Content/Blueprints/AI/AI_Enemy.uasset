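; AI controller for enemy pawns that wander the navmesh and chase the player when perceived.
; Wandering repeatedly moves to random navigable points around the pawn, chaining on each successful move.
; Perceiving a ThirdPersonCharacter starts a fast looping timer that reissues a move toward the player character.
; Losing perception only clears that timer, and wandering resumes when a chase move fails.
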(event OnTargetPerceptionUpdated(AIPerception)
  (params (Actor :type Actor%20Object%20Reference) (Stimulus :type AI%20Stimulus%20Structure))
  (Utilities|Casting|CastToThirdPersonCharacter Actor)
  (if (.bSuccessfullySensed (Utilities|Struct|BreakAIStimulus Stimulus))
    (Utilities|Time|SetTimerbyFunctionName 0 "Chase" 0.05 true)
    (else
      (Utilities|Time|ClearTimerbyFunctionName 0 "Chase"))))

(event Custom|Wander
  (AI|AIMoveTo (Pawn|GetControlledPawn) (.RandomLocation (Class|NavigationSystemV1|GetRandomPointinNavigableRadius (Transformation|GetActorLocation (Pawn|GetControlledPawn)) 1e+03 0 0)) 0 5.0 false
    (:OnSuccess
      (CallFunction|Wander))))

(event Custom|Chase
  (AI|AIMoveTo (Pawn|GetControlledPawn) "0, 0, 0" (Game|GetPlayerCharacter 0) 2e+02 false
    (:OnFail
      (CallFunction|Wander))))

(event EventBeginPlay
  (bind _asenemy_prototype (Utilities|Casting|CastToEnemyPrototype (Pawn|GetControlledPawn)))
  (Variables|Default|SetAIChar _asenemy_prototype)
  (CallFunction|Wander))

(fn ConstructionScript)